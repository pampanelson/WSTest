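; BP_grabber is a mouse-driven grabber meant to drag physics objects with a PhysicsHandle.
; Left mouse press and release call StartCarry and StopCarry, while Tick runs UpdateCarry to follow the cursor trace in X and Y at the object's current height.
; StartCarry's grab logic is disconnected from its entry and sets Carring false, as does StopCarry, so nothing shown starts a carry.
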(event `self.ReceiveTick`
  (params (DeltaSeconds :type "Float (single-precision)"))
  (`self.UpdateCarry`))

(event `Key|LeftMouseButton`
  (params (Key :type "Key Structure"))
  (:`Pressed`
    (`self.StartCarry`))
  (:`Released`
    (`self.StopCarry`)))

(fn `StartCarry`)

(fn `StopCarry`
  (`/Engine/EditorBlueprintResources/StandardMacros.IsValid` (`PhysicsHandleComponent.GetGrabbedComponent` (`self.PhysicsHandle`))
    (:`Is Valid`
      (`PhysicsHandleComponent.ReleaseComponent` (`self.PhysicsHandle`))
      (set `self.bCarring` false))))

(fn `UpdateCarry`
  (bind (_bblockinghit _binitialoverlap _time _distance _location) (`GameplayStatics.BreakHitResult` (`self.GetHitResultUnderCursorByChannel` "TraceTypeQuery1")))
  (bind (_returnvalue_x _returnvalue_y _returnvalue_z) (`KismetMathLibrary.BreakVector` (`SceneComponent.K2_GetComponentLocation` (`PhysicsHandleComponent.GetGrabbedComponent` (`self.PhysicsHandle`)))))
  (if (`self.bCarring`)
    (`PhysicsHandleComponent.SetTargetLocation` (`self.PhysicsHandle`) (`KismetMathLibrary.MakeVector` (.x _location) (.y _location) _returnvalue_z))))

(fn `UserConstructionScript`)